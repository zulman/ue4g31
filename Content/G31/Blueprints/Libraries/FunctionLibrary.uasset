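; Blueprint function library of helpers for grid-based building placement and an in-game clock.
; Cursor position comes from a line trace along the deprojected mouse ray, and GridSnap rounds a coordinate to the nearest grid step.
; SetClockWork advances a 24-hour clock by scaled delta time, returning the wrapped time and a day-rollover count.
; Two setup functions position a building's collision box and entrance just beyond the mesh's local bounds along X.
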(fn SetCursorWorldPosition
  (params (Controller :type Camera%20Pawn%20Controller%20Object%20Reference) (SightDistance :type Float%20%28single-precision%29))
  (bind (_worldlocation _worlddirection) (Game|Player|ConvertMouseLocationToWorldSpace Controller))
  (bind _outhit (Collision|LineTraceByChannel 0 _worldlocation (+ _worldlocation (* _worlddirection SightDistance)) "TraceTypeQuery3" false 0 "None"))
  (if (!= (.HitActor (Collision|BreakHitResult _outhit)) 0)
    (return (.Location (Collision|BreakHitResult _outhit)))))

(fn GridSnap
  (params (Axis :type Float%20%28single-precision%29) (GridSize :type Integer))
  (return (Math|Conversions|ToFloat(Integer) (* (Math|Float|Floor (/ (+ Axis (Math|Conversions|ToFloat(Integer) (/ GridSize 2))) (Math|Conversions|ToFloat(Integer) GridSize))) GridSize))))

(fn SetClockWork
  (params (DeltaSeconds :type Float%20%28single-precision%29) (TimeUnit :type Float%20%28single-precision%29) (ClockWork :type Float%20%28single-precision%29))
  (bind _returnvalue (/ DeltaSeconds TimeUnit))
  (bind _returnvalue_2 (+ _returnvalue ClockWork))
  (bind (_remainder _returnvalue_3) (Math|Float|Division(WholeandRemainder) _returnvalue_2 24.0))
  (return _remainder _returnvalue_3))

(fn SetBuildingCollisionBox
  (params (Collision :type Box%20Component%20Object%20Reference) (Mesh :type Static%20Mesh%20Component%20Object%20Reference))
  (bind _min (Components|StaticMesh|GetLocalBounds Mesh))
  (Components|Box|SetBoxExtent Collision (Math|Vector|MakeVector 49.0 (- (Math|Float|Absolute(Float) (.y _min)) 1e+01) 1e+01) true)
  (Transformation|SetRelativeLocation Collision (Math|Vector|MakeVector (+ (Math|Float|Absolute(Float) (.x _min)) 49.0) 0.0 1e+01) false false)
  (return))

(fn SetBuildingEntrance
  (params (Entrance :type Scene%20Component%20Object%20Reference) (Mesh :type Static%20Mesh%20Component%20Object%20Reference))
  (Transformation|SetRelativeLocation Entrance (Math|Vector|MakeVector (+ (Math|Float|Absolute(Float) (.x (.Min (Components|StaticMesh|GetLocalBounds Mesh)))) (LocalVariables|GetEntranceDistance)) 0.0 0.0) false false)
  (return))