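; Game state that runs the in-game clock and calendar and shows both on the main HUD.
; Each tick, SetClockWork advances a fractional-hour counter and yields a day tick; Clock derives hours, minutes and seconds, while Calendar rolls days into months and years.
; UpdateGameStateSpeed scales the time unit from the default speed and passes it to CallUpdateGameSpeed.
; SetClock and SetCalendar are stubs returning false.
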(event EventBeginPlay
  ;[1 1 1] Begin
  (bind _ascamera_pawn_controller (Utilities|Casting|CastToCameraPawnController (Game|GetPlayerController 0)))
  (Variables|References|SetControllerRef _ascamera_pawn_controller)
  (Variables|Default|SetClockwork (+ (Math|Conversions|ToFloat(Integer) (Variables|Default|GetHours)) (/ (Math|Conversions|ToFloat(Integer) (Variables|Default|GetMinutes)) 1.0) (/ (Math|Conversions|ToFloat(Integer) (Variables|Default|GetSeconds)) 1.0)))
  (Variables|Default|SetGameDate (Utilities|Array|MakeArray (Variables|Default|GetDay) (Variables|Default|GetMonth) (Variables|Default|GetYear)))
  (Variables|References|SetMainUIRef (Variables|/Game/G31/Blueprints/CameraPawnController.CameraPawnController_C|GetMainHudRef (Variables|References|GetControllerRef)))
  (Variables|Default|SetTimeUnit (Variables|Default|GetDefaultGameSpeed)))

(event EventTick
  (params (DeltaSeconds :type Float%20%28single-precision%29))
  ;[1 1 1] Tick
  (Variables|Default|SetClockwork (.ClockworkOut (CallFunction|SetClockWork DeltaSeconds (Variables|Default|GetTimeUnit) (Variables|Default|GetClockwork))))
  (Variables|Default|SetDayTick (.DayTick (CallFunction|SetClockWork DeltaSeconds (Variables|Default|GetTimeUnit) (Variables|Default|GetClockwork))))
  (CallFunction|Clock)
  (CallFunction|Calendar))

(event EventUpdateGameStateSpeed
  (params (Multiplier :type Float%20%28single-precision%29))
  ;[1 1 1] UpdateGameSpeed
  (bind _output_get (Variables|Default|SetTimeUnit (* (Variables|Default|GetDefaultGameSpeed) Multiplier)))
  (Default|CallUpdateGameSpeed _output_get))

(fn ConstructionScript)

(fn Clock
  (bind _clockwork (Variables|Default|GetClockwork))
  (bind _returnvalue (* _clockwork 3.6e+03))
  (bind (_remainder _returnvalue_2) (Math|Float|Division(WholeandRemainder) _returnvalue 6e+01))
  (bind _returnvalue_3 (Math|Conversions|ToFloat(Integer) _returnvalue_2))
  (bind (_remainder_2 _returnvalue_4) (Math|Float|Division(WholeandRemainder) _returnvalue_3 6e+01))
  (Variables|Default|SetSeconds (Math|Float|Floor _remainder))
  (Variables|Default|SetMinutes (Math|Float|Floor _remainder_2))
  (Variables|Default|SetHours (Math|Float|Floor (.Remainder (Math|Float|Division(WholeandRemainder) (Math|Conversions|ToFloat(Integer) _returnvalue_4) 24.0))))
  (bind _output_get (Variables|Default|SetGameTime (Utilities|Array|MakeArray (Variables|Default|GetSeconds) (Variables|Default|GetMinutes) (Variables|Default|GetHours))))
  (Class|IHUD|SetClock(Message) (Variables|References|GetMainUIRef) _output_get))

(fn Calendar
  (bind _output_get (Variables|Default|SetDay (+ (Variables|Default|GetDay) (Variables|Default|GetDayTick))))
  (if (> _output_get (Class|KismetMathLibrary|DaysinMonth (Variables|Default|GetYear) (Variables|Default|GetMonth)))
    (Variables|Default|SetDay 1)
    (Variables|Default|SetMonth (+ (Variables|Default|GetMonth) 1)))
  (if (> (Variables|Default|GetMonth) 12)
    (Variables|Default|SetMonth 1)
    (Variables|Default|SetYear (+ (Variables|Default|GetYear) 1)))
  (bind _output_get_2 (Variables|Default|SetGameDate (Utilities|Array|MakeArray (Variables|Default|GetDay) (Variables|Default|GetMonth) (Variables|Default|GetYear))))
  (Class|IHUD|SetCalendar(Message) (Variables|References|GetMainUIRef) _output_get_2))

(fn SetCalendar
  (params (Date :type Array%20of%20Integers))
  (return false))

(fn SetClock
  (params (Time :type Array%20of%20Integers))
  (return false))