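; Construction proxy actor that stands in for a building under construction, showing its display mesh with a ghost material and setting up entrance and collision.
; On BeginPlay it binds to the game state's game-speed update, with an AdjustTime event that takes a time unit.
; Each tick advances a work clock using delta time and that unit.
; When work time reaches the construction time, it broadcasts completion and destroys itself after a short delay.
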(event Custom|AdjustTime
  (params (TimeUnit :type Float%20%28single-precision%29))
  (Variables|Default|SetTimeUnit TimeUnit))

(event EventTick
  (params (DeltaSeconds :type Float%20%28single-precision%29))
  (Variables|Default|SetDelta DeltaSeconds)
  (if (not (Variables|Default|GetIsConstructionCompleted))
    (CallFunction|DoWork)
    (if (>= (Variables|Default|GetWorkTimeSpent) (Variables|Default|GetConstructionTime))
      (Variables|Default|SetIsConstructionCompleted true)
      (Default|CallConstructionCompleted self)
      (Utilities|FlowControl|Delay 0.2)
      (Actor|DestroyActor)
      (else
        (Variables|Default|SetIsConstructionCompleted false)))))

(event EventBeginPlay
  (bind _output_get (Variables|References|SetGameStateRef (.AsMy%20Game%20State (Utilities|Casting|CastToMyGameState (Game|GetGameState)))))
  (EventDispatchers|BindEventtoUpdateGameSpeed _output_get (EventDispatchers|CreateEvent :!event Custom|AdjustTime)))

(fn ConstructionScript
  (bind _staticmesh (Variables|Default|GetStaticMesh))
  (Components|StaticMesh|SetStaticMesh _staticmesh (Variables|Default|GetDisplayMesh))
  (Rendering|Material|SetMaterial _staticmesh 0 "/Game/G31/Materials/Ghost_M_Inst.Ghost_M_Inst")
  (CallFunction|SetBuildingEntrance (Variables|Default|GetEntrance) (Variables|Default|GetStaticMesh))
  (CallFunction|SetBuildingCollisionBox (Variables|Default|GetCollision) (Variables|Default|GetStaticMesh)))

(fn SetConstructionTime
  (params (ConstructionTime :type Float%20%28single-precision%29))
  (Variables|Default|SetConstructionTime (* ConstructionTime 6e+01))
  (return))

(fn DoWork
  (bind _output_get (Variables|Default|SetClockWork (.ClockworkOut (CallFunction|SetClockWork (Variables|Default|GetDelta) (Variables|Default|GetTimeUnit) (Variables|Default|GetClockWork)))))
  (Variables|Default|SetWorkTimeSpent (* _output_get 6e+01))
  (return))