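; NPC Blueprint that randomizes each character's sex, name and body color, and links to its AI controller.
; The construction script creates a dynamic body material and fills a profile with a name from per-sex name enums.
; The color branch re-rolls the random sex, so color can disagree with the stored profile.
; BeginPlay caches the NPC AI controller, through which SetIsBusy writes the blackboard's busy flag.
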(event EventBeginPlay
  (bind _returnvalue (AI|GetAIController self))
  (bind _asnpc_aicontroller_bp (Utilities|Casting|CastToNPC_AIController_BP _returnvalue))
  (Variables|References|SetAIControllerRef _asnpc_aicontroller_bp))

(fn ConstructionScript
  (CallFunction|RandomNPCFeatures))

(fn RandomNPCFeatures
  (bind _returnvalue (Math|Random|RandomIntegerinRange 0 1))
  (bind _returnvalue_2 (Math|Conversions|ToByte(Integer) _returnvalue))
  (bind _returnvalue_3 (Utilities|Enum|ByteToEnumNPSexType_ENUM _returnvalue_2))
  (bind _returnvalue_4 (Utilities|Enum|LiteralenumNPSexType_ENUM _returnvalue_3))
  (bind _returnvalue_5 (Rendering|Material|CreateDynamicMaterialInstance (Variables|Character|GetMesh) 0 "/Game/G31/Mannequin/Character/Materials/M_UE4Man_Body_Inst.M_UE4Man_Body_Inst" :!class /Script/Engine.PrimitiveComponent))
  (LocalVariables|SetMaterialInstance _returnvalue_5)
  (LocalVariables|SetRandomSex _returnvalue_4)
  (if (Utilities|Enum|Equal(Enum) _returnvalue_4 "NewEnumerator0")
    (Rendering|Material|SetVectorParameterValue (LocalVariables|GetMaterialInstance) "BodyColor" (LocalVariables|GetMaleColor) :!class /Script/Engine.MaterialInstanceDynamic)
    (else
      (Rendering|Material|SetVectorParameterValue (LocalVariables|GetMaterialInstance) "BodyColor" (LocalVariables|GetFemaleColor) :!class /Script/Engine.MaterialInstanceDynamic)))
  (bind _name (CallFunction|GetRandomName (LocalVariables|GetRandomSex)))
  (Variables|Default|SetMyProfile (Utilities|Struct|MakeNPCProfile_Struct _name (LocalVariables|GetRandomSex))))

(fn GetRandomName
  (params (Sex :type NPSexType_ENUM%20Enum))
  (if (Utilities|Enum|Equal(Enum) Sex "NewEnumerator0")
    (LocalVariables|SetSelectedName (Utilities|String|ToString(Byte) (Utilities|Enum|LiteralenumNPCName_Male_ENUM (Utilities|Enum|ByteToEnumNPCName_Male_ENUM (Math|Conversions|ToByte(Integer) (Math|Random|RandomInteger (|GetNumEnumEntries)))))))
    (else
      (LocalVariables|SetSelectedName (Utilities|String|ToString(Byte) (Utilities|Enum|LiteralenumNPCName_Female_ENUM (Utilities|Enum|ByteToEnumNPCName_Female_ENUM (Math|Conversions|ToByte(Integer) (Math|Random|RandomInteger (|GetNumEnumEntries)))))))))
  (return (LocalVariables|GetSelectedName)))

(fn SetIsBusy
  (params (Value :type Boolean))
  (AI|Components|Blackboard|SetValueasBool (AI|GetBlackboard (Variables|References|GetAIControllerRef)) (Variables|Default|GetIsBusy) Value)
  (return))